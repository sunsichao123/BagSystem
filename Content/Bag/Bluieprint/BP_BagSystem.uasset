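; Bag inventory system that stores picked-up items and shows them in a toggleable grid menu.
; On BeginPlay it builds the cell widgets, fills a parallel item array with empty slots, binds cell events and creates a hidden tooltip.
; Pickup copies a database entry by Id into the first slot with Id 0; use clears it.
; The tooltip is positioned by five-column index math and colored by rarity, though Legend reuses Epic's label.
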(event `self.ReceiveBeginPlay`
  (`self.BagInit`)
  (`self.FillItemDataArray`)
  (`self.BindCellEvent`)
  (`self.CreatItemDescript`))

(fn `BagInit`
  (bind _returnvalue (`|GenericCreateObject` "/Game/Bag/Bluieprint/UI_BagMenu.UI_BagMenu_C" self))
  (bind _output_get (set `self.BagMenu` _returnvalue))
  (`UserWidget.AddToViewport` _output_get 0)
  ;[1 1 1] 加25个bagcell
  (for _index (range (`self.Capacity`))
    (bind _returnvalue_2 (`|GenericCreateObject` "/Game/Bag/Bluieprint/UI_BagCell.UI_BagCell_C" (`self.BagMenu`)))
    (`PanelWidget.AddChild` (`/Game/Bag/Bluieprint/UI_BagMenu.CellParent` (`self.BagMenu`)) _returnvalue_2)
    (set `/Game/Bag/Bluieprint/UI_BagCell.CellIndex` _index _returnvalue_2)
    (`KismetArrayLibrary.Array_Add` (`self.BagCellArray`) _returnvalue_2))
  (`Widget.SetVisibility` (`self.BagMenu`) "Hidden"))

(fn `BindCellEvent`
  (for _array_element (`self.BagCellArray`)
    (`|ExecutionSequence`
      (:`then_0`
        (add `/Game/Bag/Bluieprint/UI_BagCell.CheckClickCellEvent` _array_element (`|CreateDelegate` :!event `UseItem`)))
      (:`then_1`
        (add `/Game/Bag/Bluieprint/UI_BagCell.HideItemDescriptionEvent` _array_element (`|CreateDelegate` :!event `HideItemDescription`)))
      (:`then_2`
        (add `/Game/Bag/Bluieprint/UI_BagCell.ShowItemDescriptionEvent` _array_element (`|CreateDelegate` :!event `ShowItemDescrition`))))))

(fn `CheckEmptyCellIndex`
  (returns (Index :type Integer))
  (for (_array_element _array_index) (`self.ItemDataArray`)
    (if (== (`.id_12_99D0DEC44C80DFC4A3852DAE9CFA0E49` (break `/Game/Bag/Bluieprint/S_Item` _array_element)) 0)
      (return _array_index)))
  (return -1))

(fn `CreatItemDescript`
  (bind _returnvalue (`|GenericCreateObject` "/Game/Bag/Bluieprint/UI_ItemDescription.UI_ItemDescription_C" self))
  (bind _output_get (set `self.ItemDescription` _returnvalue))
  (`PanelWidget.AddChild` (`/Game/Bag/Bluieprint/UI_BagMenu.ItemRoot` (`self.BagMenu`)) _output_get)
  (`Widget.SetVisibility` _output_get "Hidden"))

(fn `EnumDataByItem`
  (params (ItemLevel :type "/Game/Bag/Bluieprint/E_ItemLevel Enum" :default "NewEnumerator0"))
  (returns (`字体颜色` :type "SlateColor Structure") (levelName :type String))
  (switch `/Game/Bag/Bluieprint/E_ItemLevel` ItemLevel
    (:`NewEnumerator0`
      (return (make `SlateColor` (struct :`R` 1.0 :`G` 1.0 :`B` 1.0 :`A` 1.0)) "普通装备"))
    (:`NewEnumerator1`
      (return (make `SlateColor` (struct :`R` 0.402768 :`G` 0.474466 :`B` 1.0 :`A` 1.0)) "精良装备"))
    (:`NewEnumerator2`
      (return (make `SlateColor` (struct :`R` 0.776042 :`G` 0.028293 :`B` 0.73122 :`A` 1.0)) "史诗装备"))
    (:`NewEnumerator3`
      (return (make `SlateColor` (struct :`R` 0.902778 :`G` 0.821282 :`B` 0.117813 :`A` 1.0)) "史诗装备"))))

(fn `FillItemDataArray`
  (for _ (range (`self.Capacity`))
    (`KismetArrayLibrary.Array_Add` (`self.ItemDataArray`) (make `/Game/Bag/Bluieprint/S_Item` 0 "" "NewEnumerator0" 0 0 "NewEnumerator0" "" "/Game/Bag/Texture/cell__1_.cell__1_"))))

(fn `FindItemDataFromDataBase`
  (params (id :type Integer))
  (returns (item :type "/Game/Bag/Bluieprint/S_Item Structure"))
  (for _array_element (`self.ItemDataBase`)
    (if (== id (`.id_12_99D0DEC44C80DFC4A3852DAE9CFA0E49` (break `/Game/Bag/Bluieprint/S_Item` _array_element)))
      (return _array_element))))

(fn `HideItemDescription`
  (`Widget.SetVisibility` (`self.ItemDescription`) "Hidden"))

(fn `OpenAndCloseBag`
  (switch `ESlateVisibility` (`Widget.GetVisibility` (`self.BagMenu`))
    (:`Visible`
      (`Widget.SetVisibility` (`self.BagMenu`) "Hidden"))
    (:`Hidden`
      (`Widget.SetVisibility` (`self.BagMenu`) "Visible"))))

(fn `PickItenByID`
  (params (id :type Integer))
  (bind _item (`self.FindItemDataFromDataBase` id))
  (bind _index (`self.CheckEmptyCellIndex`))
  (if (!= _index -1)
    (bind (_id _name _type _atk _hp _level _detail _imag) (break `/Game/Bag/Bluieprint/S_Item` _item))
    (`KismetArrayLibrary.Array_Set` (`self.ItemDataArray`) _index (make `/Game/Bag/Bluieprint/S_Item` _id _name _type _atk _hp _level _detail _imag))
    (`Image.SetBrushFromTexture` (`/Game/Bag/Bluieprint/UI_BagCell.CellImage` (`|GetArrayItem` (`self.BagCellArray`) _index)) _imag false)))

(fn `ShowItemDescrition`
  (params (index :type Integer))
  (bind _itemdescription (`self.ItemDescription`))
  (bind _output (`|GetArrayItem` (`self.ItemDataArray`) index))
  (bind (_id _name _type _atk _hp _level _detail) (break `/Game/Bag/Bluieprint/S_Item` _output))
  (if (!= (`.id_12_99D0DEC44C80DFC4A3852DAE9CFA0E49` (break `/Game/Bag/Bluieprint/S_Item` _output)) 0)
    (`Widget.SetVisibility` _itemdescription "Visible")
    (`Widget.SetRenderTransform` _itemdescription (make `WidgetTransform` (+ (`KismetMathLibrary.MakeVector2D` 36.0 136.0) (`KismetMathLibrary.MakeVector2D` (+ (`KismetMathLibrary.Conv_IntToDouble` (* (mod index 5) 64)) 64.0) (+ (`KismetMathLibrary.Conv_IntToDouble` (* (/ index 5) 64)) 64.0)))))
    (bind (`_字体颜色` _levelname) (`self.EnumDataByItem` _level))
    (`/Game/Bag/Bluieprint/UI_ItemDescription.showItemDescript` (`self.ItemDescription`) `_字体颜色` _levelname _detail)))

(fn `UseItem`
  (params (index :type Integer))
  (`/Game/Bag/Bluieprint/UI_BagCell.ResetItemCell` (`|GetArrayItem` (`self.BagCellArray`) index))
  (`KismetArrayLibrary.Array_Set` (`self.ItemDataArray`) index (`self.EmptyItem`))
  (`self.HideItemDescription`))